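; Clickable recruit mini-game object that opens a player UI widget when Energy suffices, otherwise shows a throttled "No Enough Energy!!" dialog.
; Clicking increments the COFFE stat and hides the highlight, re-arming after a random delay while COFFE stays below two.
; Tick watches a separate RECURIT stat, hiding and locking the actor at five.
; Below that limit, the inherited UIReset flag zeroes RECURIT and clears the lock.
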(event EventBeginPlay
  (Variables|Default|SetEnableRank 2)
  (Variables|Default|SetDayReset true)
  (Variables|Default|SetEnableCompanyPriority true))

(event MouseInput|EventActorOnClicked
  (params (ButtonPressed :type Key%20Structure))
  (if (Variables|Default|GetIsCharactorInFrontOfObject)
    (bind _value (CallFunction|ReadStats "Energy" false))
    (if (>= _value 16.0)
      (if (not (Variables|Default|GetIsUIOpened))
        (Variables|Default|SetIsUIOpened true)
        (bind _ascharacter_base_bp (Utilities|Casting|CastToCharacterBase_BP (Game|GetPlayerCharacter 0)))
        (UserInterface|Viewport|AddtoViewport (Utilities|Array|Get(acopy) (Variables|/Game/Blueprints/CharacterBP/CharacterBase_BP.CharacterBase_BP_C|GetUIWidgetCreated _ascharacter_base_bp) 4) 0)
        (CallFunction|AddStats "COFFE" 1.0)
        (CallFunction|SetStats "ISUIOPENED" 1.0)
        (Development|SetHiddeninGame (Variables|Default|GetHighlight) true false)
        (bind _value_2 (CallFunction|ReadStats "COFFE" false))
        (if (< _value_2 2.0)
          (Utilities|FlowControl|Delay (Math|Random|RandomFloatinRange 5e+01 1e+02))
          (Development|SetHiddeninGame (Variables|Default|GetHighlight) false false)
          (Variables|Default|SetIsUIOpened false)))
      (else
        (Utilities|FlowControl|Sequence
          (:then_0
            (Utilities|FlowControl|DoOnce false :!label _label
              (:Completed
                (bind _ascharacter_base_bp_2 (Utilities|Casting|CastToCharacterBase_BP (Game|GetPlayerCharacter 0)))
                (bind _asdialog_ui (Utilities|Casting|CastToDialogUI (Utilities|Array|Get(acopy) (Variables|/Game/Blueprints/CharacterBP/CharacterBase_BP.CharacterBase_BP_C|GetUIWidgetCreated _ascharacter_base_bp_2) 8)))
                (Default|DialogtoShow _asdialog_ui "No Enough Energy!!")
                (UserInterface|Viewport|AddtoViewport _asdialog_ui 100))))
          (:then_1
            (Utilities|FlowControl|Delay 3.5)
            (goto _label Reset)))))))

(event EventTick
  (params (DeltaSeconds :type Float%20%28single-precision%29))
  (|CallParentFunction DeltaSeconds)
  (bind _value (CallFunction|ReadStats "RECURIT" false))
  (bind _output_get (Variables|Default|SetCanDo (< _value 5.0)))
  (if _output_get
    ;[1 1 1] newday
    (if (Variables|Default|GetUIReset)
      (CallFunction|SetStats "RECURIT" 0.0)
      (Variables|Default|SetIsUIOpened false)
      (Utilities|FlowControl|Delay 1.5)
      (goto _label Reset))
    (else
      (Utilities|FlowControl|DoOnce false :!label _label
        (:Completed
          (Rendering|SetActorHiddenInGame true)
          (Variables|Default|SetIsUIOpened true))))))

(fn ConstructionScript
  (|CallParentFunction))