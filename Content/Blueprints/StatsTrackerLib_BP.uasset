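; Blueprint function library that tracks named float stats stored on GameInstance_BP.
; Stats live in a Stats map, with an optional StatsMax map for upper limits, reached through a GetStats cast helper.
; NewStats registers a stat only if absent, while AddStats and SetStats change existing ones, clamping between zero and the max when one exists.
; ReadStats returns the raw value or a fraction of its max.
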(fn GetStats
  (bind _asgame_instance_bp (Utilities|Casting|CastToGameInstance_BP (Game|GetGameInstance)))
  (return _asgame_instance_bp))

(fn AddStats
  (params (StatName :type String) (Value :type Float%20%28single-precision%29))
  (bind _gameinstance (CallFunction|GetStats))
  (if (.ReturnValue (Utilities|Map|Find (Variables|/Game/Blueprints/GameInstance_BP.GameInstance_BP_C|GetStats _gameinstance) StatName))
    (if (.ReturnValue (Utilities|Map|Find (Variables|/Game/Blueprints/GameInstance_BP.GameInstance_BP_C|GetStatsMax _gameinstance) StatName))
      (Utilities|Map|Add (Variables|/Game/Blueprints/GameInstance_BP.GameInstance_BP_C|GetStats _gameinstance) StatName (Math|Float|Clamp(Float) (+ Value (.Value (Utilities|Map|Find (Variables|/Game/Blueprints/GameInstance_BP.GameInstance_BP_C|GetStats _gameinstance) StatName))) 0.0 (.Value (Utilities|Map|Find (Variables|/Game/Blueprints/GameInstance_BP.GameInstance_BP_C|GetStatsMax _gameinstance) StatName))))
      (else
        (Utilities|Map|Add (Variables|/Game/Blueprints/GameInstance_BP.GameInstance_BP_C|GetStats _gameinstance) StatName (+ Value (.Value (Utilities|Map|Find (Variables|/Game/Blueprints/GameInstance_BP.GameInstance_BP_C|GetStats _gameinstance) StatName))))))))

(fn ReadStats
  (params (StatName :type String) (ReadAsPercent :type Boolean))
  (bind _gameinstance (CallFunction|GetStats))
  (if (.ReturnValue (Utilities|Map|Find (Variables|/Game/Blueprints/GameInstance_BP.GameInstance_BP_C|GetStats _gameinstance) StatName))
    (if ReadAsPercent
      (if (.ReturnValue (Utilities|Map|Find (Variables|/Game/Blueprints/GameInstance_BP.GameInstance_BP_C|GetStatsMax _gameinstance) StatName))
        (return (/ (.Value (Utilities|Map|Find (Variables|/Game/Blueprints/GameInstance_BP.GameInstance_BP_C|GetStats _gameinstance) StatName)) (.Value (Utilities|Map|Find (Variables|/Game/Blueprints/GameInstance_BP.GameInstance_BP_C|GetStatsMax _gameinstance) StatName)))))
      (else
        (return (.Value (Utilities|Map|Find (Variables|/Game/Blueprints/GameInstance_BP.GameInstance_BP_C|GetStats _gameinstance) StatName)))))))

(fn NewStats
  (params (StatName :type String) (StartValue :type Float%20%28single-precision%29) (HaveMaxValue :type Boolean) (MaxValue :type Float%20%28single-precision%29))
  (bind _gameinstance (CallFunction|GetStats))
  (if (not (.ReturnValue (Utilities|Map|Find (Variables|/Game/Blueprints/GameInstance_BP.GameInstance_BP_C|GetStats _gameinstance) StatName)))
    (if HaveMaxValue
      (Utilities|Map|Add (Variables|/Game/Blueprints/GameInstance_BP.GameInstance_BP_C|GetStatsMax _gameinstance) StatName MaxValue))
    (Utilities|Map|Add (Variables|/Game/Blueprints/GameInstance_BP.GameInstance_BP_C|GetStats _gameinstance) StatName StartValue)))

(fn SetStats
  (params (StatName :type String) (Value :type Float%20%28single-precision%29))
  (bind _gameinstance (CallFunction|GetStats))
  (if (.ReturnValue (Utilities|Map|Find (Variables|/Game/Blueprints/GameInstance_BP.GameInstance_BP_C|GetStats _gameinstance) StatName))
    (if (.ReturnValue (Utilities|Map|Find (Variables|/Game/Blueprints/GameInstance_BP.GameInstance_BP_C|GetStatsMax _gameinstance) StatName))
      (Utilities|Map|Add (Variables|/Game/Blueprints/GameInstance_BP.GameInstance_BP_C|GetStats _gameinstance) StatName (Math|Float|Clamp(Float) Value 0.0 (.Value (Utilities|Map|Find (Variables|/Game/Blueprints/GameInstance_BP.GameInstance_BP_C|GetStatsMax _gameinstance) StatName))))
      (else
        (Utilities|Map|Add (Variables|/Game/Blueprints/GameInstance_BP.GameInstance_BP_C|GetStats _gameinstance) StatName Value)))))