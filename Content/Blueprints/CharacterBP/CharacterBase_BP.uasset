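; Base 2D side-scrolling player character with mouse and keyboard movement, door/elevator teleports and a Tab-cycled game speed.
; Holding left mouse walks to a door under the cursor, while holding right walks to the cursor point; CancelPath suspends mouse movement.
; Tick updates flipbook and facing from velocity and checks interaction overlaps for doors or quests.
; Doors are identified by actor display name, which DoorAction maps to hard-coded teleport coordinates.
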(event EventBeginPlay
  (bind _returnvalue (Game|GetPlayerController 0))
  ;[1 1 1] SetDefault
  (Variables|/Script/Engine.PlayerController|SetbEnableMouseOverEvents _returnvalue true)
  (Variables|/Script/Engine.PlayerController|SetbShowMouseCursor _returnvalue true)
  (Variables|Default|SetIsMouseInput true)
  (Variables|/Script/Engine.CharacterMovementComponent|SetMaxWalkSpeed (Variables|Character|GetCharacterMovement) (Variables|Default|GetSpeed))
  (Utilities|Time|SetGlobalTimeDilation 1.0)
  (Variables|Default|SetDoorBuildingName "None"))

(event EventTick
  (params (DeltaSeconds :type Float%20%28single-precision%29))
  (bind _ismouseinput (Variables|Default|GetIsMouseInput))
  (Utilities|FlowControl|Sequence
    (:then_0
      (CallFunction|UpdateFlipbook)
      (CallFunction|UpdateRotation)
      (CallFunction|IsInfrontOfObjectChecker))
    (:then_1
      ;[1 1 1] MouseInputMovement
      (if _ismouseinput
        (Utilities|FlowControl|Gate true
          (:Exit
            (Variables|Default|SetCanTeleport true)
            (bind (_destination _clickedactor _iscleckedondoor) (CallFunction|GetClickedLocation))
            (if _iscleckedondoor
              (CallFunction|MovetoLocatedPoint _destination)
              (if (Variables|Default|GetIsInFrontOfDoor)
                ;[1 1 1] Door Teleport
                (Utilities|IsValid _clickedactor
                  (:Is%20Valid
                    (if (Variables|Default|GetCanTeleport)
                      (Utilities|FlowControl|DoOnce false :!label _label
                        (:Completed
                          (bind _teleporttolocation (CallFunction|DoorAction (Utilities|GetDisplayName _clickedactor)))
                          (Transformation|SetActorLocation _teleporttolocation false true)
                          (Components|Movement|StopMovementImmediately (Variables|Character|GetCharacterMovement))
                          (Utilities|FlowControl|Delay 0.8)
                          (goto _label Reset))))))))))))
    (:then_2
      (if _ismouseinput
        (Utilities|FlowControl|Gate true
          (:Exit
            (Variables|Default|SetCanTeleport false)
            (bind _destionation (CallFunction|GetDestionationtoMove))
            (CallFunction|MovetoLocatedPoint _destionation)))))))

(event Input|ActionEvents|InputActionCancelPath
  (params (Key :type Key%20Structure :default "None"))
  ;[1 1 1] KeyboardInputMovement
  (:Pressed
    (Components|Movement|StopMovementImmediately (Variables|Character|GetCharacterMovement))
    (Variables|Default|SetIsMouseInput false)
    (Variables|/Script/Engine.CharacterMovementComponent|SetMaxWalkSpeed (Variables|Character|GetCharacterMovement) (Variables|Default|GetSpeed) :!label _label))
  (:Released
    (Utilities|FlowControl|Delay 0.2)
    (Variables|Default|SetIsMouseInput true)
    (goto _label)))

(event Input|AxisEvents|InputAxisKeyboardMovement
  (params (AxisValue :type Float%20%28single-precision%29))
  ;[1 1 1] KeyboardInputMovement
  (Pawn|Input|AddMovementInput "1.000000, 0, 0" AxisValue false))

(event Input|MouseEvents|RightMouseButton
  (params (Key :type Key%20Structure :default "None"))
  ;[1 1 1] MouseInputMovement
  (:Pressed
    (Utilities|FlowControl|Gate true) ; enters at Open
  )
  (:Released
    (Utilities|FlowControl|Gate true) ; enters at Close
  ))

(event Input|MouseEvents|LeftMouseButton
  (params (Key :type Key%20Structure :default "None"))
  ;[1 1 1] MouseInputMovement
  (:Pressed
    (Utilities|FlowControl|Gate true) ; enters at Open
  )
  (:Released
    (Utilities|FlowControl|Gate true) ; enters at Close
  ))

(event Input|KeyboardEvents|Tab
  (params (Key :type Key%20Structure :default "None"))
  ;[1 1 1] SetTimeDilation
  (:Pressed
    (Math|Float|CompareFloat (Variables|Default|GetTimeSpeed) 2.0
      (:>
        (Variables|Default|SetTimeSpeed 1.0))
      (:==
        (Variables|Default|SetTimeSpeed 3.0))
      (:<
        (Variables|Default|SetTimeSpeed 2.0)))
    (Utilities|Time|SetGlobalTimeDilation (Variables|Default|GetTimeSpeed))
    (Development|PrintString (Utilities|String|ToString(Float) (Variables|Default|GetTimeSpeed)))))

(fn ConstructionScript)

(fn GetDestionationtoMove
  (bind _returnvalue (Game|GetPlayerController 0))
  (bind _hitresult (Game|Player|GetHitResultUnderCursorbyChannel _returnvalue "TraceTypeQuery1" true))
  (return (Math|Vector|MakeVector (.x (.location _hitresult)) 0.0 (.z (.location _hitresult)))))

(fn MovetoLocatedPoint
  (params (Destionation :type Vector))
  (LocalVariables|SetMoveDestionation Destionation)
  (if (not (Math|Vector|Equal(Vector) (LocalVariables|GetMoveDestionation) "0, 0, 0" 0.001))
    (if (> (Math|Float|Absolute(Float) (- (.x (LocalVariables|GetMoveDestionation)) (.x (Transformation|GetActorLocation)))) 2e+01)
      (Variables|/Script/Engine.CharacterMovementComponent|SetMaxWalkSpeed (Variables|Character|GetCharacterMovement) (Variables|Default|GetSpeed))
      (AI|Navigation|SimpleMovetoLocation (Game|GetPlayerController 0) (Math|Vector|MakeVector (.x (LocalVariables|GetMoveDestionation)) 0.0 (.z (LocalVariables|GetMoveDestionation)))))))

(fn GetClickedLocation
  (bind _returnvalue (Game|GetPlayerController 0))
  (bind _hitresult (Game|Player|GetHitResultUnderCursorbyChannel _returnvalue "TraceTypeQuery3" true))
  (Utilities|IsValid (.hitactor _hitresult)
    (:Is%20Valid
      (return (Transformation|GetActorLocation (.hitactor _hitresult)) (.hitactor _hitresult) true))
    (:Is%20Not%20Valid
      (return "0.000000, 0, 0" 0 false))))

(fn MovetoActor
  (params (Actor :type Actor%20Object%20Reference))
  (AI|Navigation|SimpleMovetoActor (Game|GetPlayerController 0) Actor))

(fn UpdateFlipbook
  (LocalVariables|SetAnimationState (select (!= (Math|Vector|VectorLength (Transformation|GetVelocity)) 0.0) "NewEnumerator1" "NewEnumerator2"))
  (Sprite|SetFlipbook (Variables|Default|GetSprite) (Utilities|Select :Index (LocalVariables|GetAnimationState) :NewEnumerator0 0 :NewEnumerator1 "/Game/Assets/Sprites/Characters/Charac_Walk1.Charac_Walk1" :NewEnumerator2 "/Game/Assets/Sprites/Characters/animated_idle_charactor1.animated_idle_charactor1" :NewEnumerator3 "/Game/Assets/Sprites/Characters/Charac_Walk1.Charac_Walk1")))

(fn UpdateRotation
  (bind _sprite (Variables|Default|GetSprite))
  (Math|Float|CompareFloat (.x (Transformation|GetVelocity)) 0.0
    (:>
      (Transformation|SetRelativeRotation _sprite "0, 0, 0" false false))
    (:<
      (Transformation|SetRelativeRotation _sprite "0,180.000000, 0" false false))))

(fn DoorAction
  (params (DoorName :type String))
  (return (select (Utilities|Enum|Equal(Enum) DoorName "OutCompany") "9175.000000, 0,113.000000" (select (Utilities|Enum|Equal(Enum) DoorName "InCompany") "1969.000000, 0,144.000000" (select (Utilities|Enum|Equal(Enum) DoorName "ElevatorG") "11224.000000, 0,113.000000" (select (Utilities|Enum|Equal(Enum) DoorName "Elevator1Up") "13851.000000, 0,113.000000" (select (Utilities|Enum|Equal(Enum) DoorName "Elevator1Down") "9798.000000, 0,113.000000" (select (Utilities|Enum|Equal(Enum) DoorName "Elevator2Up") "16453.000000, 0,113.000000" (select (Utilities|Enum|Equal(Enum) DoorName "Elevator2Down") "11225.000000, 0,113.000000" (select (Utilities|Enum|Equal(Enum) DoorName "Elevator3") "13851.000000, 0,113.000000" (Transformation|GetActorLocation)))))))))))

(fn IsInfrontOfObjectChecker
  ;[1 1 1] Door
  (for _array_element (Collision|GetOverlappingActors (Variables|Default|GetInteractionHitBox) "/Game/Blueprints/BuildingDoorBP/InteractionBox_BP.InteractionBox_BP_C" :!class /Script/Engine.PrimitiveComponent)
    _)
  (if (Utilities|Enum|NotEqual(Enum) (Utilities|GetDisplayName _array_element) "")
    (if (Utilities|Array|ContainsItem (Utilities|Array|MakeArray "ElevatorG" "Elevator3" "Elevator2Up" "Elevator2Down" "Elevator1Up" "Elevator1Down" "InCompany" "OutCompany") (Utilities|GetDisplayName _array_element))
      (Variables|Default|SetIsInFrontOfDoor true)
      (else
        (Variables|Default|SetIsInFrontOfQuest true)))
    (else
      (Variables|Default|SetIsInFrontOfDoor false)
      (Variables|Default|SetIsInFrontOfQuest false))))