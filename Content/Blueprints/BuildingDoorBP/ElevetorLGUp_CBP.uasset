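; Clickable elevator door, by its name the lower-ground "up" elevator, that sets a teleport destination for the player character.
; Flags itself as a door on BeginPlay and, when clicked, writes a hardcoded world position into CharacterBase_BP's TeleportToLocation.
; When any overlap ends, it resets that target to the player's current location.
; The teleport itself is not performed in this Blueprint.
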(event EventBeginPlay
  (Variables|Default|SetIsDoor true))

(event Collision|EventActorEndOverlap
  (params (OtherActor :type Actor%20Object%20Reference))
  (bind _returnvalue (Game|GetPlayerCharacter 0))
  (bind _ascharacter_base_bp (Utilities|Casting|CastToCharacterBase_BP _returnvalue))
  (Variables|/Game/Blueprints/CharacterBP/CharacterBase_BP.CharacterBase_BP_C|SetTeleportToLocation _ascharacter_base_bp (Transformation|GetActorLocation _returnvalue)))

(event MouseInput|EventActorOnClicked
  (params (ButtonPressed :type Key%20Structure))
  (bind _ascharacter_base_bp (Utilities|Casting|CastToCharacterBase_BP (Game|GetPlayerCharacter 0)))
  (Variables|/Game/Blueprints/CharacterBP/CharacterBase_BP.CharacterBase_BP_C|SetTeleportToLocation _ascharacter_base_bp "9798.000000, 0,113.000000"))

(fn ConstructionScript
  (|CallParentFunction))