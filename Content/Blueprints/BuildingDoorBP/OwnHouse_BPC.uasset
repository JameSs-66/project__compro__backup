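; OwnHouse_BPC is a clickable building door Blueprint for the own house, which currently only reports that it is unavailable.
; On click, if the character is in front of it, it fetches the DialogUI from the player character's created-widget array and shows "No available." on screen.
; A DoOnce that resets after a short delay throttles repeated clicks.
; The construction script only calls its parent.
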(event MouseInput|EventActorOnClicked
  (params (ButtonPressed :type Key%20Structure))
  (if (Variables|Default|GetIsCharactorInFrontOfObject)
    (Utilities|FlowControl|DoOnce false :!label _label
      (:Completed
        (bind _ascharacter_base_bp (Utilities|Casting|CastToCharacterBase_BP (Game|GetPlayerCharacter 0)))
        (bind _asdialog_ui (Utilities|Casting|CastToDialogUI (Utilities|Array|Get(acopy) (Variables|/Game/Blueprints/CharacterBP/CharacterBase_BP.CharacterBase_BP_C|GetUIWidgetCreated _ascharacter_base_bp) 8)))
        (Default|DialogtoShow _asdialog_ui "No available.")
        (UserInterface|Viewport|AddtoViewport _asdialog_ui 100)
        (Utilities|FlowControl|Delay 3.5)
        (goto _label Reset)))))

(fn ConstructionScript
  (|CallParentFunction))