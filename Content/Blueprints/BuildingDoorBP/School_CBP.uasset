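; School building door Blueprint that opens the School minigame when clicked while its front-of-door area is overlapped.
; Begin and end overlap events on InFrontOfDoorCheck set and clear InfrontOfShop, which gates the click.
; A valid click adds the "School" widget from GetMiniGameWidget to the viewport and calls AddStats on ISUIOPENED to register the open UI.
; Actor overlap and construction logic defer to the parent class.
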(event OnComponentBeginOverlap(InFrontOfDoorCheck)
  (params (OverlappedComponent :type Primitive%20Component%20Object%20Reference) (OtherActor :type Actor%20Object%20Reference) (OtherComp :type Primitive%20Component%20Object%20Reference) (OtherBodyIndex :type Integer) (bFromSweep :type Boolean) (SweepResult :type Hit%20Result%20Structure%20%28by%20ref%29))
  (Variables|Default|SetInfrontOfShop true))

(event OnComponentEndOverlap(InFrontOfDoorCheck)
  (params (OverlappedComponent :type Primitive%20Component%20Object%20Reference) (OtherActor :type Actor%20Object%20Reference) (OtherComp :type Primitive%20Component%20Object%20Reference) (OtherBodyIndex :type Integer))
  (Variables|Default|SetInfrontOfShop false))

(event EventBeginPlay)

(event Collision|EventActorBeginOverlap
  (params (OtherActor :type Actor%20Object%20Reference))
  (|CallParentFunction OtherActor))

(event EventTick
  (params (DeltaSeconds :type Float%20%28single-precision%29)))

(event MouseInput|EventActorOnClicked
  (params (ButtonPressed :type Key%20Structure))
  (if (Variables|Default|GetInfrontOfShop)
    (bind _minigamewidget (CallFunction|GetMiniGameWidget "School"))
    (UserInterface|Viewport|AddtoViewport _minigamewidget 0)
    (CallFunction|AddStats "ISUIOPENED" 1.0)))

(fn ConstructionScript
  (|CallParentFunction))