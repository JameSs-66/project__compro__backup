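; Clickable employee work object that lets the player do work tasks, configured on BeginPlay with rank, company priority and next-day reset flags.
; A click in front of it with enough Energy opens a player UI widget, increments the EMWORK stat and starts a random cooldown.
; Low Energy shows a throttled warning dialog.
; Tick marks it done and blocks further work once EMWORK reaches 100 percent.
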(event EventBeginPlay
  (|CallParentFunction)
  (Variables|Default|SetEnableRank 1)
  (Variables|Default|SetResetNextDay true)
  (Variables|Default|SetEnableCompanyPriority true))

(event MouseInput|EventActorOnClicked
  (params (ButtonPressed :type Key%20Structure :default "None"))
  (if (Variables|Default|GetIsCharactorInFrontOfObject)
    (if (Variables|Default|GetCanDoQuest)
      (bind _value (CallFunction|ReadStats "Energy" false))
      (if (>= _value 8.0)
        (Variables|Default|SetCanDoQuest false)
        (bind _ascharacter_base_bp (Utilities|Casting|CastToCharacterBase_BP (Game|GetPlayerCharacter 0)))
        (UserInterface|Viewport|AddtoViewport (Utilities|Array|Get(acopy) (Variables|/Game/Blueprints/CharacterBP/CharacterBase_BP.CharacterBase_BP_C|GetUIWidgetCreated _ascharacter_base_bp) 12) 0)
        (CallFunction|SetStats "ISUIOPENED" 1.0)
        (CallFunction|AddStats "EMWORK" 1.0)
        (bind _value_2 (CallFunction|ReadStats "EMWORK" true))
        (if (!= _value_2 1.0)
          (Utilities|FlowControl|Delay (Math|Random|RandomFloatinRange 1e+01 5e+01))
          (Variables|Default|SetCanDoQuest true))
        (else
          (Utilities|FlowControl|Sequence
            (:then_0
              (Utilities|FlowControl|DoOnce false :!label _label
                (:Completed
                  (bind _ascharacter_base_bp_2 (Utilities|Casting|CastToCharacterBase_BP (Game|GetPlayerCharacter 0)))
                  (bind _asdialog_ui (Utilities|Casting|CastToDialogUI (Utilities|Array|Get(acopy) (Variables|/Game/Blueprints/CharacterBP/CharacterBase_BP.CharacterBase_BP_C|GetUIWidgetCreated _ascharacter_base_bp_2) 8)))
                  (Default|DialogtoShow _asdialog_ui "No Enough Energy!!")
                  (UserInterface|Viewport|AddtoViewport _asdialog_ui 100))))
            (:then_1
              (Utilities|FlowControl|Delay 3.5)
              (goto _label Reset))))))))

(event EventTick
  (params (DeltaSeconds :type Float%20%28single-precision%29))
  (|CallParentFunction DeltaSeconds)
  (bind _value (CallFunction|ReadStats "EMWORK" true))
  (bind _output_get (Variables|Default|SetAllDone (== _value 1.0)))
  (if _output_get
    (Variables|Default|SetCanDoQuest false)))

(fn ConstructionScript
  (|CallParentFunction))