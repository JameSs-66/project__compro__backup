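; Clickable plant pot that opens the watering-plants minigame when the character is in front with enough energy.
; Clicking hides the pot and increments the WATERPLANT stat, or shows a throttled low-energy dialog.
; Tick polls that stat, keeping the pot hidden and locked once it is full.
; While watering remains available, UIReset clears the stat and, after a delay, teleports the pot to a random hardcoded location.
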(event EventBeginPlay
  (Variables|Default|SetEnableRank 0)
  (Variables|Default|SetDayReset true)
  (Variables|Default|SetEnableCompanyPriority true)
  (Variables|Default|SetAllPlantPotLocation (Utilities|Array|MakeArray "12307.000000,-59.000000,107.000000" "12105.000000,-59.000000,107.000000" "11892.000000,-59.000000,107.000000" "12512.000000,-59.000000,107.000000" "12720.000000,-59.000000,107.000000" "16692.000000,-57.000000,110.000000" "16810.000000,-57.000000,110.000000" "17192.000000,-57.000000,110.000000" "17355.000000,-57.000000,110.000000" "17773.000000,-57.000000,110.000000" "17924.000000,-57.000000,110.000000" "18278.000000,-57.000000,110.000000" "18534.000000,-57.000000, 0")))

(event Collision|EventActorBeginOverlap
  (params (OtherActor :type Actor%20Object%20Reference))
  (|CallParentFunction OtherActor) ; This node is disabled and will not be called.\nDrag off pins to build functionality.
)

(event MouseInput|EventActorOnClicked
  (params (ButtonPressed :type Key%20Structure :default "None"))
  (if (and (Variables|Default|GetIsCharactorInFrontOfObject) (Variables|Default|GetCanDo))
    (bind _value (CallFunction|ReadStats "Energy" false))
    (if (>= _value 8.0)
      (if (not (Variables|Default|GetIsUIOpened))
        (Variables|Default|SetIsUIOpened true)
        (bind _minigamewidget (CallFunction|GetMiniGameWidget "WateringPlants_WG"))
        (UserInterface|Viewport|AddtoViewport _minigamewidget 0)
        (Rendering|SetActorHiddenInGame true)
        (CallFunction|SetStats "ISUIOPENED" 1.0)
        (CallFunction|AddStats "WATERPLANT" 1.0))
      (else
        (Utilities|FlowControl|Sequence
          (:then_0
            (Utilities|FlowControl|DoOnce false :!label _label
              (:Completed
                (bind _minigamewidget_2 (CallFunction|GetMiniGameWidget "DialogUI"))
                (bind _asdialog_ui (Utilities|Casting|CastToDialogUI _minigamewidget_2))
                (Default|DialogtoShow _asdialog_ui "No Enough Energy!!")
                (UserInterface|Viewport|AddtoViewport _minigamewidget_2 100))))
          (:then_1
            (Utilities|FlowControl|Delay 3.5)
            (goto _label Reset)))))))

(event EventTick
  (params (DeltaSeconds :type Float%20%28single-precision%29))
  (|CallParentFunction DeltaSeconds)
  (bind _value (CallFunction|ReadStats "WATERPLANT" true))
  (bind _output_get (Variables|Default|SetCanDo (!= _value 1.0)))
  (if _output_get
    ;[1 1 1] newday
    (if (Variables|Default|GetUIReset)
      (CallFunction|SetStats "WATERPLANT" 0.0)
      (Variables|Default|SetIsUIOpened false)
      (Utilities|FlowControl|Delay 1.5)
      (Transformation|SetActorLocation (.OutItem (Utilities|Array|Random (Variables|Default|GetAllPlantPotLocation))) false false)
      (goto _label Reset))
    (else
      (Utilities|FlowControl|DoOnce false :!label _label
        (:Completed
          (Rendering|SetActorHiddenInGame true)
          (Variables|Default|SetIsUIOpened true))))))

(fn ConstructionScript
  (|CallParentFunction))