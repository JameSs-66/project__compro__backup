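; VegetHealth_CBP is a clickable child Blueprint in the building-door set that opens a UI screen for the player.
; On click, if IsCharactorInFrontOfObject is true, it adds the second pre-created widget from the player's CharacterBase_BP to the viewport and sets the ISUIOPENED stat to 1.
; Begin-overlap and construction logic defer to the parent class.
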(event EventBeginPlay)

(event Collision|EventActorBeginOverlap
  (params (OtherActor :type Actor%20Object%20Reference))
  (|CallParentFunction OtherActor))

(event EventTick
  (params (DeltaSeconds :type Float%20%28single-precision%29)))

(event MouseInput|EventActorOnClicked
  (params (ButtonPressed :type Key%20Structure))
  (if (Variables|Default|GetIsCharactorInFrontOfObject)
    (bind _ascharacter_base_bp (Utilities|Casting|CastToCharacterBase_BP (Game|GetPlayerCharacter 0)))
    (UserInterface|Viewport|AddtoViewport (Utilities|Array|Get(acopy) (Variables|/Game/Blueprints/CharacterBP/CharacterBase_BP.CharacterBase_BP_C|GetUIWidgetCreated _ascharacter_base_bp) 1) 0)
    (CallFunction|SetStats "ISUIOPENED" 1.0)))

(fn ConstructionScript
  (|CallParentFunction))