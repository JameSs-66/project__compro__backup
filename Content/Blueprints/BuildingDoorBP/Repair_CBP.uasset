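; Clickable repair-job actor that opens the Repair_widget mini-game when the character is in front and has enough Energy.
; Each use increments REPAIR and, after a delay, moves the actor to a random table transform set at BeginPlay.
; Low energy shows a throttled DialogUI warning.
; Tick disables and hides it once REPAIR is full, and UIReset clears the stat while the job is available.
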(event EventBeginPlay
  (Variables|Default|SetEnableRank 0)
  (Variables|Default|SetDayReset true)
  (Variables|Default|SetEnableCompanyPriority true)
  (Variables|Default|SetAllTableLocation (Utilities|Array|MakeArray (Math|Transform|MakeTransform "9563.000000,-89.000000,671.000000" "0,-20.000000,90.000000" "1.000000,0.687500,1") (Math|Transform|MakeTransform "9336.000000,-86.000000,671.000000" "0,6.000000,90.000000" "1,0.687500,1") (Math|Transform|MakeTransform "9171.000000,-65.000000,671.000000" "0,-34.000000,90.000000" "1,0.687500,1"))))

(event Collision|EventActorBeginOverlap
  (params (OtherActor :type Actor%20Object%20Reference))
  (|CallParentFunction OtherActor) ; This node is disabled and will not be called.\nDrag off pins to build functionality.
)

(event MouseInput|EventActorOnClicked
  (params (ButtonPressed :type Key%20Structure :default "None"))
  (bind _alltablelocation (Variables|Default|GetAllTableLocation))
  (bind _outitem (Utilities|Array|Random _alltablelocation))
  (if (and (Variables|Default|GetIsCharactorInFrontOfObject) (Variables|Default|GetCanDo))
    (bind _value (CallFunction|ReadStats "Energy" false))
    (if (>= _value 8.0)
      (if (not (Variables|Default|GetIsUIOpened))
        (Variables|Default|SetIsUIOpened true)
        (bind _minigamewidget (CallFunction|GetMiniGameWidget "Repair_widget"))
        (UserInterface|Viewport|AddtoViewport _minigamewidget 0)
        (Development|SetHiddeninGame (Variables|Default|GetHighlight) true false)
        (CallFunction|SetStats "ISUIOPENED" 1.0)
        (CallFunction|AddStats "REPAIR" 1.0)
        (Utilities|FlowControl|Delay 1e+01)
        (Development|SetHiddeninGame (Variables|Default|GetHighlight) false false)
        (Transformation|SetActorLocationAndRotation (.location _outitem) (.rotation _outitem))
        (Variables|Default|SetIsUIOpened false)
        (Variables|Default|SetIsCharactorInFrontOfObject false))
      (else
        (Utilities|FlowControl|Sequence
          (:then_0
            (Utilities|FlowControl|DoOnce false :!label _label
              (:Completed
                (bind _minigamewidget_2 (CallFunction|GetMiniGameWidget "DialogUI"))
                (bind _asdialog_ui (Utilities|Casting|CastToDialogUI _minigamewidget_2))
                (Default|DialogtoShow _asdialog_ui "No Enough Energy!!")
                (UserInterface|Viewport|AddtoViewport _minigamewidget_2 100))))
          (:then_1
            (Utilities|FlowControl|Delay 3.5)
            (goto _label Reset)))))))

(event EventTick
  (params (DeltaSeconds :type Float%20%28single-precision%29))
  (|CallParentFunction DeltaSeconds)
  (bind _value (CallFunction|ReadStats "REPAIR" true))
  (bind _output_get (Variables|Default|SetCanDo (!= _value 1.0)))
  (if _output_get
    ;[1 1 1] newday
    (if (Variables|Default|GetUIReset)
      (CallFunction|SetStats "REPAIR" 0.0)
      (Variables|Default|SetIsUIOpened false)
      (Utilities|FlowControl|Delay 1.5)
      (goto _label Reset))
    (else
      (Utilities|FlowControl|DoOnce false :!label _label
        (:Completed
          (Rendering|SetActorHiddenInGame true)
          (Variables|Default|SetIsUIOpened true))))))

(fn ConstructionScript
  (|CallParentFunction))