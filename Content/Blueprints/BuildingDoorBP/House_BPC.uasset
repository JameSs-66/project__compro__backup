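; House_BPC is a clickable building door for the hotel, open only at night.
; When clicked with the character in front, it checks the WORLDTIME stat against two ranges covering the overnight window.
; During opening hours it shows a pre-created widget from the player character and sets the ISUIOPENED stat.
; Otherwise it shows the hours in DialogUI, using a DoOnce reset after a delay to block repeated messages.
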(event MouseInput|EventActorOnClicked
  (params (ButtonPressed :type Key%20Structure :default "None"))
  (if (Variables|Default|GetIsCharactorInFrontOfObject)
    (bind _value (CallFunction|ReadStats "WORLDTIME" false))
    (if (or (Math|Float|InRange(Float) _value 488.0 533.5) (Math|Float|InRange(Float) _value 0.0 111.0))
      (bind _ascharacter_base_bp (Utilities|Casting|CastToCharacterBase_BP (Game|GetPlayerCharacter 0)))
      (UserInterface|Viewport|AddtoViewport (Utilities|Array|Get(acopy) (Variables|/Game/Blueprints/CharacterBP/CharacterBase_BP.CharacterBase_BP_C|GetUIWidgetCreated _ascharacter_base_bp) 5) 25)
      (CallFunction|SetStats "ISUIOPENED" 1.0)
      (else
        (Utilities|FlowControl|DoOnce false :!label _label
          (:Completed
            (bind _ascharacter_base_bp_2 (Utilities|Casting|CastToCharacterBase_BP (Game|GetPlayerCharacter 0)))
            (bind _asdialog_ui (Utilities|Casting|CastToDialogUI (Utilities|Array|Get(acopy) (Variables|/Game/Blueprints/CharacterBP/CharacterBase_BP.CharacterBase_BP_C|GetUIWidgetCreated _ascharacter_base_bp_2) 8)))
            (Default|DialogtoShow _asdialog_ui "HOTEL is open at 22.00 - 4.00.")
            (UserInterface|Viewport|AddtoViewport _asdialog_ui 100)
            (Utilities|FlowControl|Delay 3.5)
            (goto _label Reset)))))))

(fn ConstructionScript
  (|CallParentFunction))