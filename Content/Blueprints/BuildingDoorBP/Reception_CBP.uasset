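; Reception_CBP is a child Blueprint in the building door set for a reception that stays hidden until the player becomes eligible to end the game.
; It hides itself on BeginPlay, then polls the CCEEOO stat on Tick and, once it equals 1, reveals itself and sets CanEndGame through a DoOnce.
; Clicking it while CanEndGame is set only casts the player to CharacterBase_BP, with no ending action wired.
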(event MouseInput|EventActorOnClicked
  (params (ButtonPressed :type Key%20Structure))
  (if (Variables|Default|GetCanEndGame)
    (bind _ascharacter_base_bp (Utilities|Casting|CastToCharacterBase_BP (Game|GetPlayerCharacter 0)))))

(event Collision|EventActorBeginOverlap
  (params (OtherActor :type Actor%20Object%20Reference))
  (|CallParentFunction OtherActor) ; This node is disabled and will not be called.\nDrag off pins to build functionality.
)

(event EventTick
  (params (DeltaSeconds :type Float%20%28single-precision%29))
  (bind _value (CallFunction|ReadStats "CCEEOO" false))
  (if (== _value 1.0)
    (Utilities|FlowControl|DoOnce false
      (:Completed
        (Rendering|SetActorHiddenInGame false)
        (Variables|Default|SetCanEndGame true)))))

(event EventBeginPlay
  (Rendering|SetActorHiddenInGame true)
  (Variables|Default|SetCanEndGame false))

(fn ConstructionScript
  (|CallParentFunction))