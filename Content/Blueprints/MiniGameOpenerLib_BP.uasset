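; Blueprint function library that creates and looks up minigame widgets through the Minigame map on GameInstance_BP.
; CreateMiniGameWidget instantiates each given widget class for player 0 and stores it by display name, printing a message if that key already exists.
; GetMiniGameWidget finds a widget by appending "_C_0" to the given name, relying on auto-generated instance names, and prints a message when none is found.
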(fn CreateMiniGameWidget
  (params (WidgetClass :type Array%20of%20User%20Widget%20Class%20References))
  (bind _gameinstance (CallFunction|GetMap))
  (for _array_element WidgetClass
    (bind _returnvalue (UserInterface|CreateWidget _array_element (Game|GetPlayerController 0)))
    (if (.ReturnValue (Utilities|Map|Find (Variables|/Game/Blueprints/GameInstance_BP.GameInstance_BP_C|GetMinigame _gameinstance) (Utilities|GetDisplayName _returnvalue)))
      (Development|PrintString 0 "MiniGameIsExist")
      (else
        (Utilities|Map|Add (Variables|/Game/Blueprints/GameInstance_BP.GameInstance_BP_C|GetMinigame _gameinstance) (Utilities|GetDisplayName _returnvalue) _returnvalue)))))

(fn GetMiniGameWidget
  (params (MiniGameName :type String))
  (bind _gameinstance (CallFunction|GetMap))
  (if (.ReturnValue (Utilities|Map|Find (Variables|/Game/Blueprints/GameInstance_BP.GameInstance_BP_C|GetMinigame _gameinstance) (Utilities|String|Append MiniGameName "_C_0")))
    (return (.Value (Utilities|Map|Find (Variables|/Game/Blueprints/GameInstance_BP.GameInstance_BP_C|GetMinigame _gameinstance) (Utilities|String|Append MiniGameName "_C_0"))))
    (else
      (Development|PrintString 0 "NoMiniGameExist"))))

(fn GetMap
  (bind _asgame_instance_bp (Utilities|Casting|CastToGameInstance_BP (Game|GetGameInstance)))
  (return _asgame_instance_bp))