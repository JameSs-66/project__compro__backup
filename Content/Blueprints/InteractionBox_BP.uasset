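; Interaction box actor that can be gated by company rank and re-enabled at the start of each day.
; Tick polls the CompanyRank and WORLDTIME stats to show or hide the actor and set CanInteract and UIReset.
; Cursor hover toggles a highlight through custom depth and a material swap.
; A front-of-door overlap volume flags when something stands before it; EnableAndReset is an empty stub.
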(event OnComponentBeginOverlap(InFrontOfDoorCheck)
  (params (OverlappedComponent :type Primitive%20Component%20Object%20Reference) (OtherActor :type Actor%20Object%20Reference) (OtherComp :type Primitive%20Component%20Object%20Reference) (OtherBodyIndex :type Integer) (bFromSweep :type Boolean) (SweepResult :type Hit%20Result%20Structure%20%28by%20ref%29))
  (if (Variables|Default|GetCanInteract)
    (Variables|Default|SetIsCharactorInFrontOfObject true)))

(event OnComponentEndOverlap(InFrontOfDoorCheck)
  (params (OverlappedComponent :type Primitive%20Component%20Object%20Reference) (OtherActor :type Actor%20Object%20Reference) (OtherComp :type Primitive%20Component%20Object%20Reference) (OtherBodyIndex :type Integer))
  (Variables|Default|SetIsCharactorInFrontOfObject false))

(event EventTick
  (params (DeltaSeconds :type Float%20%28single-precision%29))
  (if (Variables|Default|GetEnableCompanyPriority)
    (bind _value (CallFunction|ReadStats "CompanyRank" false))
    (if (== (Math|Float|Truncate _value) (Variables|Default|GetEnableRank))
      (if (Variables|Default|GetDayReset) :!label _label
        (bind _value_2 (CallFunction|ReadStats "WORLDTIME" false))
        (if (Math|Float|InRange(Float) _value_2 0.0 0.5)
          (goto _label_2 Reset)
          (else
            (Variables|Default|SetUIReset false)
            (Utilities|FlowControl|DoOnce true :!label _label_2
              (:Completed
                (Rendering|SetActorHiddenInGame false)
                (Variables|Default|SetUIReset true)
                (Variables|Default|SetCanInteract true))))))
      (else
        (Variables|Default|SetCanInteract false)
        (Rendering|SetActorHiddenInGame true)))
    (else
      (goto _label))))

(event MouseInput|EventActorBeginCursorOver
  (bind _highlight (Variables|Default|GetHighlight))
  (Rendering|SetRenderCustomDepth _highlight true)
  (Rendering|Material|SetMaterial _highlight 0 "/Game/Blueprints/BuildingDoorBP/Materials/DoorFrame_M.DoorFrame_M"))

(event MouseInput|EventActorEndCursorOver
  (bind _highlight (Variables|Default|GetHighlight))
  (Rendering|SetRenderCustomDepth _highlight false)
  (Rendering|Material|SetMaterial _highlight 0 "/Game/Blueprints/BuildingDoorBP/Materials/Invisible_M.Invisible_M"))

(fn ConstructionScript)

(fn EnableandReset
  (params (EnableOnRank :type Integer) (EnableDayReset :type Boolean)))