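; Clock Blueprint whose hour and minute hands display the in-game time.
; Every tick it reads the WORLDTIME stat and converts it into whole minute and hour steps.
; Each step sets the pitch of its hand in world space, so the hands jump in discrete increments and ignore the actor's own rotation.
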(event EventTick
  (params (DeltaSeconds :type Float%20%28single-precision%29))
  (bind _value (CallFunction|ReadStats "WORLDTIME" false))
  (Transformation|SetWorldRotation (Variables|Default|GetMinHand) (Math|Rotator|MakeRotator 0.0 (Math|Conversions|ToFloat(Integer) (* (Math|Integer|%(Integer) (Math|Float|Truncate (/ _value 0.37)) 60) -6)) 0.0) false false)
  (Transformation|SetWorldRotation (Variables|Default|GetHourHand) (Math|Rotator|MakeRotator 0.0 (* (Math|Float|Truncate (/ _value 22.200001)) -3e+01) 0.0) false false))

(fn ConstructionScript)